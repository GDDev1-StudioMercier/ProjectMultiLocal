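; BP_OndeDeChoc is a shockwave actor that expands once on spawn and ragdolls players caught in it.
; The Grow timeline drives the ShockWave component's X and Y scale outward at a fixed height.
; Overlapping BP_ThirdPersonCharacterQAM characters call Ragdoll only if their CanHide flag is true.
; When growth finishes, it destroys itself and calls RespawningMessage(false) on four player characters.
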(event `self.ReceiveBeginPlay`
  (bind (_direction _growing) (`Timeline|Grow` :!via `PlayFromStart`)
    (:`Update`
      (bind _returnvalue (* _growing 200.0))
      (`SceneComponent.SetRelativeScale3D` (`self.ShockWave`) (`KismetMathLibrary.MakeVector` _returnvalue _returnvalue 5.0)))
    (:`Finished`
      (`self.K2_DestroyActor`)
      (for _index (range 4)
        (message `/Game/GR2_QAM/BluePrint/BPI_Respawn.Respawning` (`GameplayStatics.GetPlayerCharacter` _index) false)))))

(event `self.ShockWave.OnComponentBeginOverlap`
  (params (OverlappedComponent :type "PrimitiveComponent Object Reference") (OtherActor :type "Actor Object Reference") (OtherComp :type "PrimitiveComponent Object Reference") (OtherBodyIndex :type Integer) (bFromSweep :type Boolean) (SweepResult :type "HitResult Structure (by ref)"))
  (bind _asbp_third_person_character_qam (cast `/Game/GR2_QAM/Players/BP_ThirdPersonCharacterQAM` OtherActor))
  (if (`/Game/GR2_QAM/Players/BP_ThirdPersonCharacterQAM.bCanHide?` _asbp_third_person_character_qam)
    (`/Game/GR2_QAM/Players/BP_ThirdPersonCharacterQAM.Ragdoll` _asbp_third_person_character_qam)))

(fn `UserConstructionScript`)