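; Game manager actor that ends a multiplayer match when only one player remains.
; At BeginPlay it creates the end-game widget and reads the player count, minus one, from the QAM game mode.
; Each EndGame call decrements that count; at zero it finds the character not flagged dead, stores it as winner and assigns a hardcoded name by array index.
; It then pauses the game, shows the widget and switches input to UI only.
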(event `self.ReceiveBeginPlay`
  (bind _returnvalue (`|CreateWidget` "/Game/GR2_QAM/Widget/WBP_EndGame.WBP_EndGame_C"))
  (set `self.HUDRef_EndGame` _returnvalue)
  (bind _asbp_third_person_game_mode_qam (cast `/Game/GR2_QAM/Players/BP_ThirdPersonGameModeQAM` (`GameplayStatics.GetGameMode`)))
  (set `self.nbPlayers` (- (`/Game/GR2_QAM/Players/BP_ThirdPersonGameModeQAM.NbPlayers` _asbp_third_person_game_mode_qam) 1)))

(event `EndGame`
  (bind _result (`/Engine/EditorBlueprintResources/StandardMacros.DecrementInt` (`self.nbPlayers`))
    (:`  `
      (if (<= _result 0)
        (bind _outactors (`GameplayStatics.GetAllActorsOfClass` "/Game/GR2_QAM/Players/BP_ThirdPersonCharacterQAM.BP_ThirdPersonCharacterQAM_C"))
        (for (_array_element _array_index) _outactors
          (if (not (`/Game/GR2_QAM/Players/BP_ThirdPersonCharacterQAM.bIsDead` _array_element))
            (set `self.BPRef_Winner` _array_element)
            (switch `int` _array_index
              (:`0`
                (set `self.PlayerName` "Guillaume"))
              (:`1`
                (set `self.PlayerName` "Hervé"))
              (:`2`
                (set `self.PlayerName` "René"))
              (:`3`
                (set `self.PlayerName` "Pronto")))))
        (`GameplayStatics.SetGamePaused` true)
        (`UserWidget.AddToViewport` (`self.HUDRef_EndGame`) 0)
        (`WidgetBlueprintLibrary.SetInputMode_UIOnlyEx` (`GameplayStatics.GetPlayerController` 0) null)))))

(fn `UserConstructionScript`)