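; BP_Marteau is a hammer actor that periodically smashes a random tile of the game grid.
; A looping timer picks a tile from RedGridManager and removes it from the grid.
; Chained timelines sweep the hammer above it, lower it, and pitch the mesh, with the swing restarted on each descent update.
; After impact, it spawns a BP_OndeDeChoc shockwave, messages the tile to fall, then lerps back to its initial transform.
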(event `self.ReceiveBeginPlay`
  (set `self.InitialTransform` (`SceneComponent.K2_GetComponentToWorld` (`self.DefaultSceneRoot`)))
  (`KismetSystemLibrary.K2_SetTimerDelegate` (delegate `Event Bonk`) (`self.TimeBetweenBonks`) true))

(event `Event Bonk`
  (bind (_returnvalue_x _returnvalue_y _returnvalue_z) (`KismetMathLibrary.BreakVector` (`self.K2_GetActorLocation`)))
  (bind (_newpos_x _newpos_y) (`KismetMathLibrary.BreakVector` (`self.NewPos`)))
  (bind (_initialtransform_location _initialtransform_rotation) (`KismetMathLibrary.BreakTransform` (`self.InitialTransform`)))
  (bind _returnvalue (`SceneComponent.K2_GetComponentLocation` (`self.DefaultSceneRoot`)))
  ; Choisit aléatoirement une case
  (bind _grille (`/Game/GR2_QAM/BluePrint/BP_gridManager.GetRandomGrille` (`self.RedGridManager`)))
  (bind _output_get (set `self.Grille` _grille))
  (`KismetArrayLibrary.Array_RemoveItem` (`/Game/GR2_QAM/BluePrint/BP_gridManager.grilleDeJeu` (`self.RedGridManager`)) _output_get)
  (bind (_returnvalue_x_2 _returnvalue_y_2 _returnvalue_z_2) (`KismetMathLibrary.BreakVector` (`self.K2_GetActorLocation` _grille)))
  (set `self.NewPos` (`KismetMathLibrary.MakeVector` (+ _returnvalue_x_2 400.0) _returnvalue_y_2 (+ _returnvalue_z_2 240.0)))
  ; Se déplace vers la case
  (bind (_direction _bonkzone) (`Timeline|SweepToBonkZone` :!via `PlayFromStart`)
    (:`Update`
      (`self.K2_SetActorLocation` (`KismetMathLibrary.VLerp` (`KismetMathLibrary.MakeVector` _returnvalue_x _returnvalue_y _returnvalue_z) (`KismetMathLibrary.MakeVector` _newpos_x _newpos_y _returnvalue_z) _bonkzone) true))
    (:`Finished`
      ; Se déplace vers le bas
      (bind (_direction_2 _descending) (`Timeline|Descend` :!via `PlayFromStart`)
        (:`Update`
          (`self.K2_SetActorLocation` (`KismetMathLibrary.VLerp` _returnvalue (- _returnvalue (0.0 0.0 14.75)) _descending) true)
          ; Animation de Bonk
          (bind (_direction_3 _bonk) (`Timeline|Bonk` :!via `PlayFromStart`)
            (:`Update`
              (`SceneComponent.K2_SetRelativeRotation` (`self.StaticMesh`) (`KismetMathLibrary.MakeRotator` 0.0 (* _bonk 90.0)) false false))
            (:`Finished`
              ; Spawn de l'onde de choc
              (`|SpawnActorFromClass` "/Game/GR2_QAM/BluePrint/BP_OndeDeChoc.BP_OndeDeChoc_C" (`KismetMathLibrary.MakeTransform` (`SceneComponent.K2_GetComponentLocation` (`self.Collision`))) "AlwaysSpawn" "MultiplyWithRoot" null null)
              ; Appel d'un Interact - Tomber la case
              (message `/Game/GR2_QAM/BluePrint/BPI_CaseFalling.FallingCase` (`self.Grille`))
              ; Retour à la position de départ
              (bind (_direction_4 _goback) (`Timeline|InitialPosition` :!via `PlayFromStart`)
                (:`Update`
                  (`self.K2_SetActorLocation` (`KismetMathLibrary.VLerp` (`SceneComponent.K2_GetComponentLocation` (`self.DefaultSceneRoot`)) _initialtransform_location _goback) true)
                  (`SceneComponent.K2_SetRelativeRotation` (`self.StaticMesh`) (`KismetMathLibrary.RLerp` (`SceneComponent.K2_GetComponentRotation` (`self.StaticMesh`)) _initialtransform_rotation _goback) false false))))))))))

(fn `UserConstructionScript`)