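; BP_gridManager builds the square game board at BeginPlay by spawning a grid of BP_GrilleDeJeu cell actors.
; Two nested loops over the side length (LongeurCote) place cells TailleCase apart, row by row from positive to negative Y.
; A computed offset centers the board on the world origin, independent of the manager's location.
; Each spawned cell is appended to the GrilleDeJeu array.
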(event `self.ReceiveBeginPlay`
  (bind _taillecase (`self.tailleCase`))
  (bind _taillecase_2 (`self.tailleCase`))
  (bind _returnvalue (`KismetMathLibrary.FTrunc` (`self.worldOffSet`)))
  ; pour changer la taille des cases :metter la taille de la case dans la variable du même nom puis changer la longeur d'un coté si vous le souhaiter (ce programme ne permet que de faire des carré)
  (set `self.worldOffset` (- (* (* (`self.longeurCote`) _taillecase) 0.5) (* _taillecase 0.5)))
  (for _index (range (`self.longeurCote`))
    (for _index_2 (range (`self.longeurCote`))
      (bind _returnvalue_2 (`|SpawnActorFromClass` "/Game/GR2_QAM/BluePrint/BP_GrilleDeJeu.BP_GrilleDeJeu_C" (`KismetMathLibrary.MakeTransform` (`KismetMathLibrary.MakeVector` (`KismetMathLibrary.Conv_IntToDouble` (- (* _index_2 _taillecase_2) _returnvalue)) (`KismetMathLibrary.Conv_IntToDouble` (- _returnvalue (* _taillecase_2 _index))))) "AlwaysSpawn" "MultiplyWithRoot" null null))
      (`KismetArrayLibrary.Array_Add` (`self.grilleDeJeu`) _returnvalue_2))))

(fn `UserConstructionScript`)