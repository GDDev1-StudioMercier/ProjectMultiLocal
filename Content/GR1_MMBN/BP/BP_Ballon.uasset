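; BP_Ballon is the physics ball of a two-team scoring game, and it also tracks both scores and the win condition.
; It saves its starting transform and velocity at BeginPlay, restores them on Spawn while re-enabling scoring, and moves by impulse when kicked.
; IncrementScore updates the score widget, then CheckScore shows the victory widget with UI-only input once either team reaches three points.
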(event `self.ReceiveBeginPlay`
  (bind _ballon (`self.Ballon`))
  (`|ExecutionSequence`
    (:`then_0`
      ; Etat intial de la balle
      (`self.InitialTransformBallon`))
    (:`then_1`
      (`PrimitiveComponent.SetSimulatePhysics` _ballon true)
      (`PrimitiveComponent.SetEnableGravity` _ballon true))))

(event `CreateWBPSCore`
  ;[1 0.15 0.15 0.5] Création du Widget Score
  (bind _returnvalue (`|GenericCreateObject` "/Game/GR1_MMBN/BP/WBP/WBP_Score.WBP_Score_C"))
  (bind _output_get (set `self.WBP_Score` _returnvalue))
  (`UserWidget.AddToViewport` _output_get 0))

(event `InitialTransformBallon`
  (bind _ballon (`self.Ballon`))
  ;[0 0 0 0.5] Etat de base de la balle en début de jeu [Mehdy]
  (set `self.Position_Initial` (`SceneComponent.GetRelativeTransform` _ballon))
  (set `self.Velocity_Initial` (`SceneComponent.GetComponentVelocity` _ballon)))

(event `Spawn`
  (bind _velocity_initial (`self.Velocity_Initial`))
  ;[0 0 0 0.5] Respawn de la balle + stop mouvment [Mehdy]
  (`SceneComponent.K2_SetWorldTransform` (`self.Ballon`) (`self.Position_Initial`) false true)
  (`PrimitiveComponent.SetPhysicsLinearVelocity` (`self.Ballon`) _velocity_initial false "None")
  (`PrimitiveComponent.SetPhysicsAngularVelocityInDegrees` (`self.Ballon`) _velocity_initial false "None")
  (set `self.CanScore` true))

(event `IncrementScore`
  (params (TeamA :type Boolean))
  ;[0 0 0 0.5] Systeme de points [Mehdy]
  (bind _result (`/Engine/EditorBlueprintResources/StandardMacros.IncrementInt` (select `bool` TeamA :`false` (`self.Score_TB`) :`true` (`self.Score_TA`)))
    (:`  `
      (`/Game/GR1_MMBN/BP/WBP/WBP_Score.UpdateScore` (`self.WBP_Score`) _result TeamA)
      (`self.CheckScore`))))

(event `/Game/GR1_MMBN/Player/BPI_Kick.Kick`
  (params (Direction :type "Vector Structure"))
  ;[0.15 1 0.05859 0.5] Kick du ballon
  (`PrimitiveComponent.AddImpulse` (`self.Ballon`) (* Direction (`self.Kick_Strength_ballon`)) "None" true))

(event `CheckScore`
  (bind _returnvalue (`GameplayStatics.GetPlayerController` 0))
  (bind _wbp_victoire (`self.WBP_Victoire`))
  ;[0.15 0.15 1 0.5] Condition de Victoire et affichage
  (if (or (>= (`self.Score_TB`) 3) (>= (`self.Score_TA`) 3))
    (bind _returnvalue_2 (`|GenericCreateObject` "/Game/GR1_MMBN/BP/WBP/WBP_Victoire.WBP_Victoire_C"))
    (bind _output_get (set `self.WBP_Victoire` _returnvalue_2))
    (`UserWidget.AddToViewport` _output_get 0)
    (`WidgetBlueprintLibrary.SetInputMode_UIOnlyEx` _returnvalue (`self.WBP_Victoire`))
    (set `PlayerController.bShowMouseCursor` true _returnvalue)
    (`Widget.RemoveFromParent` (`self.WBP_Score`))
    (if (>= (`self.Score_TB`) 3)
      (`/Game/GR1_MMBN/BP/WBP/WBP_Victoire.TeamBWin` _wbp_victoire)
      (else
        (`/Game/GR1_MMBN/BP/WBP/WBP_Victoire.TeamAWin` _wbp_victoire)))))

(fn `UserConstructionScript`)