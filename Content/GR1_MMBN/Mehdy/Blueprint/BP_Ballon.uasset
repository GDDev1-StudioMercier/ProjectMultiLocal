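; BP_Ballon is the game ball, with respawn and score counting for two sides, A and B.
; On BeginPlay it saves the Ballon component's relative transform and velocity.
; Spawn teleports it to that saved transform, applied in world space, and reuses the saved velocity for both linear and angular physics velocity to stop its motion.
; IncrementScoreA and IncrementScoreB raise their counters and tell the Score object to update.
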(event `self.ReceiveBeginPlay`
  (`self.Stat`))

(event `Stat`
  (bind _ballon (`self.Ballon`))
  ;[0 0 0 0.5] Etat de base de la balle en début de jeu [Mehdy]
  (set `self.Position_Initial` (`SceneComponent.GetRelativeTransform` _ballon))
  (set `self.Velocity_Initial` (`SceneComponent.GetComponentVelocity` _ballon)))

(event `Spawn`
  (bind _velocity_initial (`self.Velocity_Initial`))
  ;[0 0 0 0.5] Respawn de la balle + stop mouvment [Mehdy]
  (`SceneComponent.K2_SetWorldTransform` (`self.Ballon`) (`self.Position_Initial`) false true)
  (`PrimitiveComponent.SetPhysicsLinearVelocity` (`self.Ballon`) _velocity_initial false "None")
  (`PrimitiveComponent.SetPhysicsAngularVelocityInDegrees` (`self.Ballon`) _velocity_initial false "None"))

(event `IncrementScoreA`
  (`/Engine/EditorBlueprintResources/StandardMacros.IncrementFloat` (`self.Score_TA`)
    (:`  `
      (`/Game/GR1_MMBN/Mehdy/Widget_BP/WBP_Score.UpdateScoreA` (`self.Score`)))))

(event `IncrementScoreB`
  (`/Engine/EditorBlueprintResources/StandardMacros.IncrementFloat` (`self.Score_TB`)
    (:`  `
      (`/Game/GR1_MMBN/Mehdy/Widget_BP/WBP_Score.UpdateScoreB` (`self.Score`)))))

(fn `UserConstructionScript`)