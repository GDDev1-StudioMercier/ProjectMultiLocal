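; BP_KABWLOOWYYYY is a thrown gift bomb that explodes on a timer and knocks back AMKY third-person characters.
; Launch_Kaboom silences Sphere1 collision, launches DemomanGift with a physics impulse and soon arms damage.
; Five seconds later it plays the explosion, briefly waits, then switches the sphere to overlap and immediately destroys itself.
; Armed overlaps with characters apply a hugely scaled velocity impulse; the stored thrower is never checked.
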(event `Launch_Kaboom`
  (params (direction :type "Vector Structure") (`Who throw it` :type "Actor Object Reference"))
  (bind _demomangift (`self.DemomanGift`))
  (`PrimitiveComponent.SetCollisionResponseToAllChannels` (`self.Sphere1`) "ECR_Ignore")
  (set `self.Who Throw It` `Who throw it`)
  (`PrimitiveComponent.SetSimulatePhysics` (`self.DemomanGift`) true)
  (`PrimitiveComponent.AddImpulse` (`self.DemomanGift`) direction "None" true)
  (`KismetSystemLibrary.Delay` 0.1)
  (set `self.canDamage` true)
  (`KismetSystemLibrary.Delay` 5.0)
  (`GameplayStatics.SpawnEmitterAttached` "/Game/StarterContent/Particles/P_Explosion.P_Explosion" _demomangift "None" (`SceneComponent.RelativeLocation` _demomangift) (struct) (10.0 10.0 10.0) "KeepWorldPosition")
  (`GameplayStatics.PlaySound2D` "/Game/StarterContent/Audio/Explosion01.Explosion01" 1.0 1.0 0.0 null null)
  (`KismetSystemLibrary.Delay` 0.2)
  (`PrimitiveComponent.SetCollisionResponseToAllChannels` (`self.Sphere1`) "ECR_Overlap")
  (`self.K2_DestroyActor`))

(event `self.Sphere1.OnComponentBeginOverlap`
  (params (OverlappedComponent :type "PrimitiveComponent Object Reference") (OtherActor :type "Actor Object Reference") (OtherComp :type "PrimitiveComponent Object Reference") (OtherBodyIndex :type Integer) (bFromSweep :type Boolean) (SweepResult :type "HitResult Structure (by ref)"))
  (if (`self.canDamage`)
    (cast `/Game/GR3_AMKY/Matthias/BP/BP_KABWLOOWYYYY` OtherActor
      (:`CastFailed`
        (bind _asbp_third_person_character_amky (cast `/Game/GR3_AMKY/core/Players/BP_ThirdPersonCharacterAMKY` OtherActor))
        (`KismetSystemLibrary.PrintString` (`KismetSystemLibrary.GetDisplayName` OtherActor))
        (`/Game/GR3_AMKY/core/Players/BP_ThirdPersonCharacterAMKY.take impulse` _asbp_third_person_character_amky (* (`self.GetVelocity`) 10000000))
        (`self.K2_DestroyActor`)))))

(fn `UserConstructionScript`)