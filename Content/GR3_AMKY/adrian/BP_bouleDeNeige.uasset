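; BP_bouleDeNeige is a thrown snowball projectile that knocks back characters it strikes.
; The launchsnowball event stores the thrower, enables physics on Sphere and applies the given direction as a velocity-change impulse.
; A Sphere1 overlap with anything but another snowball destroys it and passes its scaled velocity to BP_ThirdPersonCharacterAMKY's TakeImpulse.
; Any Sphere hit also destroys it, and the stored thrower is never checked.
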(event `launch snowball`
  (params (direction :type "Vector Structure") (WhoThrowIt :type "Actor Object Reference"))
  (set `self.Who Throw It` WhoThrowIt)
  (`PrimitiveComponent.SetSimulatePhysics` (`self.Sphere`) true)
  (`PrimitiveComponent.AddImpulse` (`self.Sphere`) direction "None" true))

(event `self.Sphere1.OnComponentBeginOverlap`
  (params (OverlappedComponent :type "PrimitiveComponent Object Reference") (OtherActor :type "Actor Object Reference") (OtherComp :type "PrimitiveComponent Object Reference") (OtherBodyIndex :type Integer) (bFromSweep :type Boolean) (SweepResult :type "HitResult Structure (by ref)"))
  (cast `/Game/GR3_AMKY/adrian/BP_bouleDeNeige` OtherActor
    (:`CastFailed`
      (`self.K2_DestroyActor`)
      (bind _asbp_third_person_character_amky (cast `/Game/GR3_AMKY/core/Players/BP_ThirdPersonCharacterAMKY` OtherActor))
      (`/Game/GR3_AMKY/core/Players/BP_ThirdPersonCharacterAMKY.take impulse` _asbp_third_person_character_amky (* (`self.GetVelocity`) 100)))))

(event `self.Sphere.OnComponentHit`
  (params (HitComponent :type "PrimitiveComponent Object Reference") (OtherActor :type "Actor Object Reference") (OtherComp :type "PrimitiveComponent Object Reference") (NormalImpulse :type "Vector Structure") (Hit :type "HitResult Structure (by ref)"))
  (`self.K2_DestroyActor`))

(fn `UserConstructionScript`)